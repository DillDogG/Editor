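; BP_Turret is a turret actor that rotates steadily and scans for actors in front of it.
; Tick yaws the Scene component at RotationRate, scaled by delta time.
; A looping half-second timer runs a Visibility line trace from the Arrow along its forward vector for Distance.
; On a hit it only prints the actor's name and draws a debug sphere at the impact point.
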(event `self.ReceiveBeginPlay`
  (`KismetSystemLibrary.K2_SetTimerDelegate` (delegate `LineTrace`) 0.5 true))

(event `LineTrace`
  (bind _arrow (`self.Arrow`))
  (bind _returnvalue (`SceneComponent.K2_GetComponentLocation` _arrow))
  (bind _outhit (`KismetSystemLibrary.LineTraceSingle` _returnvalue (+ _returnvalue (* (`SceneComponent.GetForwardVector` _arrow) (`self.Distance`))) "TraceTypeQuery1"))
  (bind (_bblockinghit _binitialoverlap _time _distance _location _impactpoint _normal _impactnormal _physmat _hitactor) (`GameplayStatics.BreakHitResult` _outhit))
  (`/Engine/EditorBlueprintResources/StandardMacros.IsValid` _hitactor
    (:`Is Valid`
      (`KismetSystemLibrary.PrintString` (`KismetSystemLibrary.GetDisplayName` _hitactor))
      (`KismetSystemLibrary.DrawDebugSphere` _location))))

(event `self.ReceiveTick`
  (params (DeltaSeconds :type "Float (single-precision)"))
  (`SceneComponent.K2_AddRelativeRotation` (`self.Scene`) (`KismetMathLibrary.MakeRotator` 0.0 0.0 (* DeltaSeconds (`self.RotationRate`))) false false))

(fn `UserConstructionScript`)