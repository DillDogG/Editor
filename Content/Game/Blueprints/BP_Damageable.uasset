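; BP_Damageable is a short-lived actor that damages whatever overlaps it and can itself be destroyed for points.
; It sets a brief lifespan on BeginPlay and applies its Damage to overlapping actors.
; Incoming damage runs through an ApplyDamage helper, fed a literal zero health rather than the Health variable, which stores the result.
; When the helper reports destruction, it adds Points to the ShooterInstance game instance and destroys the actor.
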(event `self.ReceiveBeginPlay`
  (`self.SetLifeSpan` 2.0))

(event `self.ReceiveActorBeginOverlap`
  (params (OtherActor :type "Actor Object Reference"))
  (`GameplayStatics.ApplyDamage` OtherActor (`self.Damage`) null self))

(event `self.ReceiveAnyDamage`
  (params (Damage :type "Float (single-precision)") (DamageType :type "DamageType Object Reference") (InstigatedBy :type "Controller Object Reference") (DamageCauser :type "Actor Object Reference"))
  (bind (_outhealth _destroyed) (`/Game/Game/Blueprints/NewFunctionLibrary.ApplyDamage` 0.0 Damage))
  (set `self.Health` _outhealth)
  (if _destroyed
    (bind _asshooter_instance (cast `/Game/Game/Blueprints/ShooterInstance` (`GameplayStatics.GetGameInstance`)))
    (`/Game/Game/Blueprints/ShooterInstance.AddPoints` _asshooter_instance (`self.Points`))
    (`self.K2_DestroyActor`)))

(fn `UserConstructionScript`)